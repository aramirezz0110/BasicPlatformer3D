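; Enemy is a moving hazard actor that damages the player's MyCharacter on overlap.
; On BeginPlay it stores its start location, then a timeline offsets it from that point along either its X or Y track, chosen by the MovementInX flag.
; Overlapping MyCharacter applies a fixed amount of damage, with movement done through non-swept location updates.
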(event `self.ReceiveBeginPlay`
  (bind _output_get (set `self.EnemyPosition` (`self.K2_GetActorLocation`)))
  (bind (_direction _xmove _ymove) (`Timeline|EnemyMovementTimeline`)
    (:`Update`
      (if (`self.MovementInX`)
        (`self.K2_SetActorLocation` (+ _xmove _output_get))
        (else
          (`self.K2_SetActorLocation` (+ _ymove _output_get)))))))

(event `self.ReceiveActorBeginOverlap`
  (params (OtherActor :type "Actor Object Reference"))
  (bind _asmy_character (cast `/Game/Blueprints/Game/MyCharacter` OtherActor))
  (`GameplayStatics.ApplyDamage` _asmy_character 10.0))

(fn `UserConstructionScript`)