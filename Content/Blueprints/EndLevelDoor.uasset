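; End-level door actor that the player can open with the UseObject input after collecting three items.
; Box overlap checks MyCharacter's Collectables and shows a timed TextAlert prompt through ShowAlertMessage, enabling door input after the delay only if the count equals three.
; Leaving the box disables input.
; Pressing UseObject plays a timeline that offsets the door's yaw from its rotation at that press.
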(event `InputAction|UseObject`
  (params (Key :type "Key Structure"))
  ;[1 1 1] Open Door using a key input action
  (:`Pressed`
    (bind _output_get (set `self.InitialRotation` (`self.K2_GetActorRotation`)))
    (bind (_direction _opendoortrack) (`Timeline|OpenDoorTimeline`)
      (:`Update`
        (`self.K2_SetActorRotation` (`KismetMathLibrary.MakeRotator` (.roll _output_get) (.pitch _output_get) (- (.yaw _output_get) _opendoortrack)))))))

(event `self.ReceiveBeginPlay`)

(event `self.Box.OnComponentBeginOverlap`
  (params (OverlappedComponent :type "PrimitiveComponent Object Reference") (OtherActor :type "Actor Object Reference") (OtherComp :type "PrimitiveComponent Object Reference") (OtherBodyIndex :type Integer) (bFromSweep :type Boolean) (SweepResult :type "HitResult Structure (by ref)"))
  (set `self.openDoorAvailable` true)
  (bind _asmy_character (cast `/Game/Blueprints/Game/MyCharacter` OtherActor))
  (if (== (`/Game/Blueprints/Game/MyCharacter.Collectables` _asmy_character) 3)
    (`self.ShowAlertMessage` _asmy_character "Press F to open the door" 1.0
      (:`Output`
        (`self.EnableInput` (`GameplayStatics.GetPlayerController` 0))))
    (else
      (`self.ShowAlertMessage` _asmy_character "You need to collect 3 items!" 1.0
        (:`Output`
          (`self.DisableInput` (`GameplayStatics.GetPlayerController` 0) :!label _label))))))

(event `self.Box.OnComponentEndOverlap`
  (params (OverlappedComponent :type "PrimitiveComponent Object Reference") (OtherActor :type "Actor Object Reference") (OtherComp :type "PrimitiveComponent Object Reference") (OtherBodyIndex :type Integer))
  (set `self.openDoorAvailable` false)
  (cast `/Game/Blueprints/Game/MyCharacter` OtherActor)
  (goto _label))

(fn `UserConstructionScript`)