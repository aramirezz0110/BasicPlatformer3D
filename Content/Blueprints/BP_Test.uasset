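; BP_Test is a scratch Blueprint demonstrating basic scripting: variables, branches, loops, switches, functions, events and macros.
; Each topic has its own graph printing test variables, but none are wired to execution and BeginPlay is empty.
; The construction script sets the test float and integer.
; A delayed sequence compares MyFunction, MyEvent and MyMacro running the same print loop, where function and macro exit on the first iteration.
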(event `self.ReceiveBeginPlay`)

(event `MyEvent`
  (if (`self.TestBoolean`)
    (for _ (range 5)
      (`KismetSystemLibrary.PrintString` "MyEvent"))))

(fn `MyFunction`
  (params (NewParam :type String))
  (returns (NewParam1 :type Boolean))
  (if (`self.TestBoolean`)
    (for _ (range 5)
      (`KismetSystemLibrary.PrintString` "MyFunction!")
      (return (`self.TestBoolean`)))))

(fn `TestFunction`)

(fn `UserConstructionScript`
  (set `self.TestFloat` 6.9)
  (set `self.TestInt` 69))