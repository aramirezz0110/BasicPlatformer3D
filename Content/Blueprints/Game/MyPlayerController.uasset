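; MyPlayerController is a player controller that turns player input into movement, look, jump and pause actions for the player's character.
; On BeginPlay it casts the player character to MyCharacter and stores it for the input handlers to drive.
; Movement follows the forward and right vectors of the full control rotation, and look axes feed pitch and yaw input.
; The pause action toggles game pause, and both it and jump print debug messages.
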(event `InputAction|JumpAction`
  (params (Key :type "Key Structure"))
  ;[1 1 1] View movement
  (:`Pressed`
    (`Character.Jump` (`self.My Character`))
    (`KismetSystemLibrary.PrintString` "Jump!")))

(event `self.ReceiveBeginPlay`
  (bind _asmy_character (cast `/Game/Blueprints/Game/MyCharacter` (`GameplayStatics.GetPlayerCharacter` 0)))
  (set `self.My Character` _asmy_character))

(event `InputAction|Pause` :paused true
  (params (Key :type "Key Structure"))
  ;[1 1 1] Set game state
  (:`Pressed`
    (if (`GameplayStatics.IsGamePaused`)
      (`GameplayStatics.SetGamePaused` false)
      (`KismetSystemLibrary.PrintString` "Game in play mode")
      (else
        (`GameplayStatics.SetGamePaused` true)
        (`KismetSystemLibrary.PrintString` "Game Paused")))))

(event `InputAxis|LookUpDown`
  (params (AxisValue :type "Float (single-precision)"))
  ;[1 1 1] View movement
  (`Pawn.AddControllerPitchInput` (`self.My Character`) AxisValue))

(event `InputAxis|LookRightLeft`
  (params (AxisValue :type "Float (single-precision)"))
  ;[1 1 1] View movement
  (`Pawn.AddControllerYawInput` (`self.My Character`) AxisValue))

(event `InputAxis|MovingForwardBackward`
  (params (AxisValue :type "Float (single-precision)"))
  (bind _my_character (`self.My Character`))
  ;[1 1 1] Forward and Backward movement
  (`Pawn.AddMovementInput` _my_character (`KismetMathLibrary.GetForwardVector` (`Pawn.GetControlRotation` _my_character)) AxisValue false))

(event `InputAxis|MovingRightLeft`
  (params (AxisValue :type "Float (single-precision)"))
  (bind _my_character (`self.My Character`))
  ;[1 1 1] Right and Left movement
  (`Pawn.AddMovementInput` _my_character (`KismetMathLibrary.GetRightVector` (`Pawn.GetControlRotation` _my_character)) AxisValue false))

(fn `UserConstructionScript`)