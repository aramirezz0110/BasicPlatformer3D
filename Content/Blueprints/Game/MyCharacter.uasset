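; Player character Blueprint that tracks health and a collectable count, reporting both as on-screen debug prints.
; Incoming damage passes through a DoOnce that resets after a short delay, creating brief invulnerability between hits.
; At zero health it prints a death message and leaves the gate closed, without calling game over.
; Separate custom events increment collectables and quit the game on game over.
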(event `self.ReceiveAnyDamage`
  (params (Damage :type "Float (single-precision)") (DamageType :type "DamageType Object Reference") (InstigatedBy :type "Controller Object Reference") (DamageCauser :type "Actor Object Reference"))
  (`/Engine/EditorBlueprintResources/StandardMacros.DoOnce` false :!label _label
    (:`Completed`
      (bind _output_get (set `self.Health` (- (`self.Health`) Damage)))
      (`KismetSystemLibrary.PrintString` (`KismetStringLibrary.Concat_StrStr` "Health: " (`KismetStringLibrary.Conv_DoubleToString` _output_get)))
      (if (> _output_get 0.0)
        (`KismetSystemLibrary.PrintString` "Receiving damage!")
        (`KismetSystemLibrary.Delay` 0.5)
        (goto _label :!via `Reset`)
        (else
          (`KismetSystemLibrary.PrintString` "You Died"))))))

(event `IncreaseCollectable`
  (bind _output_get (set `self.Collectables` (+ (`self.Collectables`) 1)))
  (`KismetSystemLibrary.PrintString` (`KismetStringLibrary.Concat_StrStr` "Collectables: " (`KismetStringLibrary.Conv_IntToString` _output_get))))

(event `EventGameOver`
  (`KismetSystemLibrary.QuitGame` null "Quit"))

(fn `UserConstructionScript`)